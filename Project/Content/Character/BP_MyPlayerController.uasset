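; Player controller for building placement, enabling placement mode on BeginPlay or B and spawning buildings on left click through SpawnBuilding and SpawnBuilding1.
; Blueprint "1" functions manage a preview actor, snap it to CV_GridManager's grid via mouse trace, and spawn copies when SV_PloppableComponent reports valid placement.
; SetPlacementModeEnabled1 is never called and both update calls are disconnected from Tick.
; The unsuffixed functions are defined outside this file.
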(event `self.ReceiveBeginPlay`
  (`self.SetPlacementModeEnabled` true :!label _label))

(event `Key|B`
  (params (Key :type "Key Structure"))
  (:`Pressed`
    (goto _label)))

(event `self.ReceiveTick`
  (params (DeltaSeconds :type "Float (single-precision)")))

(event `Key|LeftMouseButton`
  (params (Key :type "Key Structure"))
  (:`Pressed`
    (if (`self.PlacementModeEnabled`)
      (`self.SpawnBuilding`)
      (`self.SpawnBuilding1`))))

(fn `SetPlacementModeEnabled1`
  (params (`Is Enabled` :type Boolean))
  (bind _placeableactor_0 (`self.PlaceableActor_0`))
  (if (== `Is Enabled` (`self.PlacementModeEnabled_0`))
    (return)
    (else
      (bind _output_get (set `self.PlacementModeEnabled_0` `Is Enabled`))
      (if _output_get
        (bind _returnvalue (`|SpawnActorFromClass` (`self.PlaceableActorType_0`) (`KismetMathLibrary.MakeTransform` (0.0 0.0 -100000.0)) "AlwaysSpawn" "OverrideRootScale" null null))
        (bind _output_get_2 (set `self.PlaceableActor_0` _returnvalue))
        (bind _returnvalue_2 (`self.GetComponentByClass` _output_get_2 "/Game/GameObjects/Components/SV_ClickableComponent.SV_ClickableComponent_C"))
        (`/Engine/EditorBlueprintResources/StandardMacros.IsValid` _returnvalue_2
          (:`Is Valid`
            (`/Game/GameObjects/Components/SV_ClickableComponent.InPlacementMode` _returnvalue_2))
          (:`Is Not Valid`
            _))
        (`AddComponent|NODE_AddSV_PloppableComponent-0` :`self` _output_get_2)
        (else
          (`/Engine/EditorBlueprintResources/StandardMacros.IsValid` _placeableactor_0
            (:`Is Valid`
              (`self.K2_DestroyActor` _placeableactor_0))))))))

(fn `SpawnBuilding1`
  (bind _returnvalue (`self.GetComponentByClass` (`self.PlaceableActor_0`) "/Game/GameObjects/Components/SV_PloppableComponent.SV_PloppableComponent_C"))
  (`/Engine/EditorBlueprintResources/StandardMacros.IsValid` _returnvalue
    (:`Is Valid`
      (if (`/Game/GameObjects/Components/SV_PloppableComponent.IsPlacementValid` _returnvalue)
        (`|SpawnActorFromClass` (`self.PlaceableActorType_0`) (`self.GetTransform` (`self.PlaceableActor_0`)) "AlwaysSpawn" "OverrideRootScale" null null)))))

(fn `UpdatePlacement1`
  (bind (_worldlocation _worlddirection) (`self.DeprojectMousePositionToWorld`))
  (bind _outhit (`KismetSystemLibrary.LineTraceSingle` _worldlocation (+ _worldlocation (* _worlddirection 100000.0)) "TraceTypeQuery3"))
  (bind (_bblockinghit _binitialoverlap _time _distance _location) (`GameplayStatics.BreakHitResult` _outhit))
  (if _bblockinghit
    (bind _returnvalue (`GameplayStatics.GetActorOfClass` "/Game/GameObjects/Grid/CV_GridManager.CV_GridManager_C"))
    (bind _outputvector (`/Game/GameObjects/Grid/CV_GridManager.GetClossetGridPosition` _returnvalue _location))
    (`self.K2_SetActorLocation` (`self.PlaceableActor_0`) _outputvector false false)))

(fn `UserConstructionScript`)