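; Player controller Blueprint that owns the building menu UI and lets the player toggle it.
; On BeginPlay it creates the BuildingMenu widget, stores it, adds it to the viewport and hides it.
; Pressing B runs a FlipFlop that alternates the menu between visible and hidden.
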(event `self.ReceiveBeginPlay`
  (bind _returnvalue (`|CreateWidget` "/Game/UI/BuildingMenu.BuildingMenu_C"))
  (bind _output_get (set `self.BuildingMenu` _returnvalue))
  (`UserWidget.AddToViewport` _output_get 0)
  (`Widget.SetVisibility` (`self.BuildingMenu`) "Hidden"))

(event `Key|B`
  (params (Key :type "Key Structure"))
  (:`Pressed`
    (`/Engine/EditorBlueprintResources/StandardMacros.FlipFlop`
      (:`A`
        (`Widget.SetVisibility` (`self.BuildingMenu`) "Visible"))
      (:`B`
        (`Widget.SetVisibility` (`self.BuildingMenu`) "Hidden")))))

(fn `UserConstructionScript`)