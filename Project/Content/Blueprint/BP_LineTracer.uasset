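; BP_LineTracer is an actor that probes static world geometry with a line trace to read the surface angle.
; BeginPlay sets a fixed rotation, then each Tick traces for WorldStatic objects along the Sphere component's forward vector, with debug drawing.
; It stores the hit actor's display name in HitActor and the normal's X and Y in GroundAngle.
; The closing zero-normal checks trigger nothing.
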(event `self.ReceiveBeginPlay`
  (`self.K2_SetActorRotation` (struct :`Pitch` -90.0)))

(event `self.ReceiveTick`
  (params (DeltaSeconds :type "Float (single-precision)"))
  (bind _sphere (`self.Sphere`))
  (bind _returnvalue (`SceneComponent.K2_GetComponentLocation` _sphere))
  (bind _outhit (`KismetSystemLibrary.LineTraceSingleForObjects` :`Start` _returnvalue :`End` (+ _returnvalue (* (`KismetMathLibrary.GetForwardVector` (`SceneComponent.K2_GetComponentRotation` _sphere)) (10000.0 10000.0 10000.0))) :`ObjectTypes` (`|MakeArray` "ObjectTypeQuery1" :!type "EObjectTypeQuery Enum") :`DrawDebugType` "ForOneFrame"))
  (bind (_bblockinghit _binitialoverlap _time _distance _location _impactpoint _normal _impactnormal _physmat _hitactor) (`GameplayStatics.BreakHitResult` _outhit))
  (set `self.HitActor` (`KismetSystemLibrary.GetDisplayName` _hitactor))
  (set `self.GroundAngle` (`KismetMathLibrary.MakeRotator` (.x _normal) (.y _normal)))
  (if (== (* (.x _normal) 180.0) 0.0)
    (if (== (* (.y _normal) 180.0) 0.0)
      _)))

(fn `UserConstructionScript`)