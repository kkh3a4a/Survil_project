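; BP_Spawn_Sun_Detecter is a spawner actor that lays out a square grid of BP_LineTrace_Ground actors, apparently for sun detection.
; On BeginPlay it stores its root's world location, then nested inclusive loops offset X and Y by Distance, giving OneSideMax + 1 actors per side at the same height.
; Any grid point where the spawn would collide is skipped.
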(event `self.ReceiveBeginPlay`
  (bind _distance (`self.Distance`))
  (bind (_locationspwaned_x _locationspwaned_y _locationspwaned_z) (`KismetMathLibrary.BreakVector` (`self.LocationSpwaned`)))
  (bind _onesidemax (`self.OneSideMax`))
  (set `self.LocationSpwaned` (`SceneComponent.K2_GetComponentLocation` (`self.DefaultSceneRoot`)))
  (for _index (range (+ _onesidemax 1))
    (for _index_2 (range (+ _onesidemax 1))
      (`|SpawnActorFromClass` "/Game/Blueprint/BP_LineTrace_Ground.BP_LineTrace_Ground_C" (`KismetMathLibrary.MakeTransform` (`KismetMathLibrary.MakeVector` (+ (* _index_2 _distance) _locationspwaned_x) (+ (* _index _distance) _locationspwaned_y) _locationspwaned_z)) "DontSpawnIfColliding" "OverrideRootScale" null null))))

(fn `UserConstructionScript`)