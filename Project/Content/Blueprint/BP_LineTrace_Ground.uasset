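; Debug actor that line-traces against WorldStatic objects and reports the surface normal it hits.
; BeginPlay snaps the actor to a fixed rotation, then every Tick casts a long ray from the Sphere component along its forward vector.
; The trace is drawn for one frame and the hit normal is printed on screen, without checking whether anything was hit.
; An unconnected set-location-and-rotation node and an empty branch never run.
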(event `self.ReceiveBeginPlay`
  (`self.K2_SetActorRotation` (struct :`Pitch` -90.0)))

(event `self.ReceiveTick`
  (params (DeltaSeconds :type "Float (single-precision)"))
  (bind _sphere (`self.Sphere`))
  (bind _returnvalue (`SceneComponent.K2_GetComponentLocation` _sphere))
  (bind _outhit (`KismetSystemLibrary.LineTraceSingleForObjects` :`Start` _returnvalue :`End` (+ _returnvalue (* (`KismetMathLibrary.GetForwardVector` (`SceneComponent.K2_GetComponentRotation` _sphere)) (10000.0 10000.0 10000.0))) :`ObjectTypes` (`|MakeArray` "ObjectTypeQuery1" :!type "EObjectTypeQuery Enum") :`DrawDebugType` "ForOneFrame"))
  (bind (_bblockinghit _binitialoverlap _time _distance _location _impactpoint _normal) (`GameplayStatics.BreakHitResult` _outhit))
  (`KismetSystemLibrary.PrintString` (`KismetStringLibrary.Conv_VectorToString` (`KismetMathLibrary.MakeVector` (.x _normal) (.y _normal) (.z _normal))) true true (struct :`R` 1.0 :`G` 0.038955 :`A` 1.0)))

(fn `UserConstructionScript`)