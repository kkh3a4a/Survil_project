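; BP_Food is a food resource actor that removes itself from the world when its server-side resource entry runs out.
; Every Tick it finds the Server_testing actor and loops over the values of its ResourcesCreateLandscape map.
; It selects its entry by matching the array index to the last index of its own Tags array, so tag count encodes identity.
; It destroys itself when that entry's Count is zero or less.
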(event `self.ReceiveTick`
  (params (DeltaSeconds :type "Float (single-precision)"))
  (bind _returnvalue (`GameplayStatics.GetActorOfClass` "/Script/Project.Server_testing"))
  (bind _values (`BlueprintMapLibrary.Map_Values` (`Server_testing.resources_create_landscape` _returnvalue)))
  (for (_array_element _array_index) _values
    (if (== (`KismetArrayLibrary.Array_LastIndex` (`self.Tags`)) _array_index)
      (if (<= (`.count` (break `resources_actor` _array_element)) 0)
        (`self.K2_DestroyActor`)))))

(fn `UserConstructionScript`)