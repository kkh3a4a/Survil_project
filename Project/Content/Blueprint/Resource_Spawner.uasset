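; Resource spawner actor that populates the landscape with oil, water, iron, food and tree actors from data held by the Server_testing actor.
; On its first Tick it loops over the server's ResourcesCreateLandscape values, spawning the matching Blueprint at each X/Y with Z at zero.
; Each spawn is tagged "Resource" plus its type.
; A flag prevents respawning, even if that data was empty, though the server lookup repeats every Tick.
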(event `self.ReceiveBeginPlay`
  (set `self.first_recv_send` false)
  (bind _returnvalue (`GameplayStatics.GetActorOfClass` "/Script/Project.Server_testing"))
  (set `self.server` _returnvalue))

(event `self.ReceiveTick`
  (params (DeltaSeconds :type "Float (single-precision)"))
  (bind _returnvalue (`GameplayStatics.GetActorOfClass` "/Script/Project.Server_testing"))
  (bind _output_get (set `self.server` _returnvalue))
  (if (not (`self.first_recv_send`))
    (bind _values (`BlueprintMapLibrary.Map_Values` (`Server_testing.resources_create_landscape` _output_get)))
    (for _array_element _values
      (bind (_type _count _location) (break `resources_actor` _array_element))
      (if (== _type 0)
        (bind _returnvalue_2 (`|SpawnActorFromClass` "/Game/Blueprint/Resource/BP_Oil.BP_Oil_C" (`KismetMathLibrary.MakeTransform` (`KismetMathLibrary.MakeVector` (break `three_float` _location) (`.y` (break `three_float` _location)) 0.0)) "Undefined" "OverrideRootScale" null null))
        (set `Actor.Tags` (`|MakeArray` "Resource" (`KismetStringLibrary.Conv_StringToName` (`KismetStringLibrary.Conv_IntToString` _type))) _returnvalue_2)
        (elif (== _type 1)
          (bind _returnvalue_3 (`|SpawnActorFromClass` "/Game/Blueprint/Resource/BP_Water.BP_Water_C" (`KismetMathLibrary.MakeTransform` (`KismetMathLibrary.MakeVector` (break `three_float` _location) (`.y` (break `three_float` _location)) 0.0)) "Undefined" "OverrideRootScale" null null))
          (set `Actor.Tags` (`|MakeArray` "Resource" (`KismetStringLibrary.Conv_StringToName` (`KismetStringLibrary.Conv_IntToString` _type))) _returnvalue_3)
          (elif (== _type 2)
            (bind _returnvalue_4 (`|SpawnActorFromClass` "/Game/Blueprint/Resource/BP_Iron.BP_Iron_C" (`KismetMathLibrary.MakeTransform` (`KismetMathLibrary.MakeVector` (break `three_float` _location) (`.y` (break `three_float` _location)) 0.0)) "Undefined" "OverrideRootScale" null null))
            (set `Actor.Tags` (`|MakeArray` "Resource" (`KismetStringLibrary.Conv_StringToName` (`KismetStringLibrary.Conv_IntToString` _type))) _returnvalue_4)
            (elif (== _type 3)
              (bind _returnvalue_5 (`|SpawnActorFromClass` "/Game/Blueprint/Resource/BP_Food.BP_Food_C" (`KismetMathLibrary.MakeTransform` (`KismetMathLibrary.MakeVector` (break `three_float` _location) (`.y` (break `three_float` _location)) 0.0)) "Undefined" "OverrideRootScale" null null))
              (set `Actor.Tags` (`|MakeArray` "Resource" (`KismetStringLibrary.Conv_StringToName` (`KismetStringLibrary.Conv_IntToString` _type))) _returnvalue_5)
              (elif (== _type 4)
                (bind _returnvalue_6 (`|SpawnActorFromClass` "/Game/Blueprint/Resource/BP_Tree.BP_Tree_C" (`KismetMathLibrary.MakeTransform` (`KismetMathLibrary.MakeVector` (break `three_float` _location) (`.y` (break `three_float` _location)) 0.0)) "Undefined" "OverrideRootScale" null null))
                (set `Actor.Tags` (`|MakeArray` "Resource" (`KismetStringLibrary.Conv_StringToName` (`KismetStringLibrary.Conv_IntToString` _type))) _returnvalue_6)))))))
    (set `self.first_recv_send` true)))

(fn `UserConstructionScript`)