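; Landscape test actor that spawns a square grid of PlaneTile actors when play begins.
; Two nested loops over OneSideNumber offset each tile along X and Y by multiples of Distance from the root component's world location, keeping its Z.
; The grid starts one Distance away from the spawner, and tiles that would collide are not spawned.
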(event `self.ReceiveBeginPlay`
  (bind (_locationspawned_x _locationspawned_y _locationspawned_z) (`KismetMathLibrary.BreakVector` (`self.LocationSpawned`)))
  (bind _distance (`self.Distance`))
  (bind _onesidenumber (`self.OneSideNumber`))
  (set `self.LocationSpawned` (`SceneComponent.K2_GetComponentLocation` (`self.DefaultSceneRoot`)))
  (for _index (range 1 (+ _onesidenumber 1))
    (for _index_2 (range 1 (+ _onesidenumber 1))
      (`|SpawnActorFromClass` "/Game/Blueprint/LandscapeTest/PlaneTile.PlaneTile_C" (`KismetMathLibrary.MakeTransform` (`KismetMathLibrary.MakeVector` (+ (* _index_2 _distance) _locationspawned_x) (+ (* _index _distance) _locationspawned_y) _locationspawned_z)) "DontSpawnIfColliding" "OverrideRootScale" null null))))

(fn `UserConstructionScript`)