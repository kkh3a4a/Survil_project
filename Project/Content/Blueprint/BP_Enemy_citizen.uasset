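; BP_Enemy_citizen is an enemy citizen actor whose position mirrors data held by the Server_testing actor.
; Every Tick it matches its second tag against the keys of the server's Citizen map to set MyTeam.
; Its third tag indexes CitizenLocationRotation in the map value whose position equals MyTeam.
; It moves to that entry's X and Y at a fixed height, leaving rotation unapplied.
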(event `self.ReceiveTick`
  (params (DeltaSeconds :type "Float (single-precision)"))
  (bind _returnvalue (`GameplayStatics.GetActorOfClass` "/Script/Project.Server_testing"))
  (for (_array_element _array_index) (`self.Tags`)
    (if (== _array_index 1)
      (bind _keys (`BlueprintMapLibrary.Map_Keys` (`Server_testing.citizen` _returnvalue)))
      (for _array_element_2 _keys
        (if (== _array_element_2 (`KismetStringLibrary.Conv_NameToString` _array_element))
          (set `self.myTeam` _array_element_2)))
      (elif (== _array_index 2)
        (bind _values (`BlueprintMapLibrary.Map_Values` (`Server_testing.citizen` _returnvalue)))
        (for (_array_element_3 _array_index_2) _values
          (if (== (`self.myTeam`) _array_index_2)
            (for (_array_element_4 _array_index_3) (`.citizen_location_rotation` (break `citizen_struct` _array_element_3))
              (if (== _array_index_3 (`KismetStringLibrary.Conv_StringToInt` (`KismetStringLibrary.Conv_NameToString` _array_element)))
                (bind _location (break `Citizen_sole` _array_element_4))
                (`self.K2_SetActorLocation` (`KismetMathLibrary.MakeVector` (break `three_float` _location) (`.y` (break `three_float` _location)) 100.0))))))))))

(fn `UserConstructionScript`)