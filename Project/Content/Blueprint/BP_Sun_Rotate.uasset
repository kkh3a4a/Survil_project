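; Sun actor that rotates continuously on pitch to drive a day cycle, starting from a fixed angle at BeginPlay.
; Each Tick advances SunAngle by SunMoveInTick, or subtracts 360 without advancing when the next step would reach 360.
; Outside the wrap, the applied pitch runs one extra step ahead of the stored angle.
; The Daylight flag is true while SunAngle exceeds 180.
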(event `self.ReceiveBeginPlay`
  (set `self.Sun Angle` 200.0))

(event `self.ReceiveTick`
  (params (DeltaSeconds :type "Float (single-precision)"))
  (bind _returnvalue (+ (`self.Sun Angle`) (`self.Sun Move In Tick`)))
  (if (>= _returnvalue 360.0)
    (bind _output_get (set `self.Sun Angle` (- (`self.Sun Angle`) 360.0)))
    (`self.K2_SetActorRotation` (`KismetMathLibrary.MakeRotator` 0.0 _output_get))
    (else
      (set `self.Sun Angle` _returnvalue)
      (`self.K2_SetActorRotation` (`KismetMathLibrary.MakeRotator` 0.0 _returnvalue))))
  (set `self.Daylight` (> (`self.Sun Angle`) 180.0)))

(fn `UserConstructionScript`)