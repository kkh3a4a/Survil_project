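; Test actor that builds a square grid of sand tiles as instances on the Sands instanced mesh component.
; BeginPlay adds SandsSize by SandsSize unit-scale instances spaced 100 units apart.
; A disconnected loop would set each instance's Z scale from GetHeight using a row-major index, but it never runs.
; Tick and the construction script are empty, so the grid stays flat.
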(event `self.ReceiveBeginPlay`
  (bind _returnvalue (- (`self.sands_size`) 1))
  (for _index (range (+ _returnvalue 1))
    (for _index_2 (range (+ _returnvalue 1))
      (`InstancedStaticMeshComponent.AddInstance` (`self.sands`) (`KismetMathLibrary.MakeTransform` (`KismetMathLibrary.MakeVector` (`KismetMathLibrary.Conv_IntToDouble` (* _index_2 100)) (`KismetMathLibrary.Conv_IntToDouble` (* _index 100))) (struct) (1.0 1.0 1.0)) false))))

(event `self.ReceiveTick`
  (params (DeltaSeconds :type "Float (single-precision)")))

(fn `UserConstructionScript`)