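; Test actor, apparently for sand, that builds a square grid of height-varying columns with a Hierarchical Instanced Static Mesh.
; Nested loops over SandsSize place evenly spaced instances, taking each Z scale from IntArray with a hard-coded row stride of 10.
; The construction script builds the grid, and Tick repeats the same loops every frame without clearing, so instances keep accumulating.
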(event `self.ReceiveTick`
  (params (DeltaSeconds :type "Float (single-precision)"))
  (bind _sands_size (`self.sands_size`))
  (for _index (range (+ _sands_size 1))
    (for _index_2 (range (+ _sands_size 1))
      (`InstancedStaticMeshComponent.AddInstance` (`self.HierarchicalInstancedStaticMesh`) (`KismetMathLibrary.MakeTransform` (`KismetMathLibrary.MakeVector` (`KismetMathLibrary.Conv_IntToDouble` (* _index 50)) (`KismetMathLibrary.Conv_IntToDouble` (* _index_2 50))) (struct) (`KismetMathLibrary.MakeVector` 1.0 1.0 (`KismetMathLibrary.Conv_IntToDouble` (`|GetArrayItem` (`self.IntArray`) (+ (* _index 10) _index_2))))) false))))

(fn `UserConstructionScript`
  (bind _sands_size (`self.sands_size`))
  (for _index (range (+ _sands_size 1))
    (for _index_2 (range (+ _sands_size 1))
      (`InstancedStaticMeshComponent.AddInstance` (`self.HierarchicalInstancedStaticMesh`) (`KismetMathLibrary.MakeTransform` (`KismetMathLibrary.MakeVector` (`KismetMathLibrary.Conv_IntToDouble` (* _index 50)) (`KismetMathLibrary.Conv_IntToDouble` (* _index_2 50))) (struct) (`KismetMathLibrary.MakeVector` 1.0 1.0 (`KismetMathLibrary.Conv_IntToDouble` (`|GetArrayItem` (`self.IntArray`) (+ (* _index 10) _index_2))))) false))))