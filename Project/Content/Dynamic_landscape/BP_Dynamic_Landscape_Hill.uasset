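; Hill actor for a dynamic landscape that stamps the M_Hill material into a shared render target, which it clears to white on BeginPlay.
; On Cleared_RT, separate X and Y checks stamp when outside the central dead zone but within outer bounds, otherwise hide the actor.
; Stamping raises the actor, traces down to the Landscape, then draws at the normalized hit position, scaled by relative actor scale.
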(event `self.ReceiveBeginPlay`
  (set `self.Render Material` "/Game/LandScape_change_test/mater/M_Hill.M_Hill")
  (`KismetRenderingLibrary.ClearRenderTarget2D` "/Game/Dynamic_landscape/Dynamic_render_target.Dynamic_render_target" (struct :`R` 1.0 :`G` 1.0 :`B` 1.0 :`A` 1.0)))

(event `self.ReceiveTick`
  (params (DeltaSeconds :type "Float (single-precision)")))

(event `Cleared_RT`
  (bind _returnvalue (`self.K2_GetActorLocation`))
  (bind (_returnvalue_x _returnvalue_y) (`KismetMathLibrary.BreakVector` (`self.K2_GetActorLocation`)))
  (bind _landscape (`self.Landscape`))
  (bind (_returnvalue_x_2 _returnvalue_y_2) (`KismetMathLibrary.BreakVector` (`self.K2_GetActorLocation` _landscape)))
  (bind (_origin _boxextent) (`self.GetActorBounds` _landscape false false))
  (bind _returnvalue_2 (+ _returnvalue_x 0.0))
  (bind _returnvalue_3 (+ _returnvalue_y 0.0))
  (bind _returnvalue_x_3 (`KismetMathLibrary.BreakVector` (/ (`self.GetActorScale3D`) (`self.GetActorScale3D` (`self.Landscape`)))))
  (if (> _returnvalue_x -25000.0)
    (if (< _returnvalue_x 25000.0)
      (if (> _returnvalue_y -25000.0)
        (if (< _returnvalue_y 25000.0)
          (`|ExecutionSequence`
            (:`then_0`
              (if (> _returnvalue_x 8000.0)
                (`self.SetActorHiddenInGame` false :!label _label)
                (`self.K2_SetActorLocation` (`KismetMathLibrary.MakeVector` _returnvalue_2 _returnvalue_3 10000.0))
                (bind (_outhit _returnvalue_4) (`KismetSystemLibrary.LineTraceSingle` :`Start` (+ _returnvalue (0.0 0.0 0.0)) :`End` (- _returnvalue (0.0 0.0 100000.0)) :`TraceChannel` "TraceTypeQuery1" :`DrawDebugType` "ForOneFrame"))
                (bind _aslandscape (cast `Landscape` (`.HitActor` (`GameplayStatics.BreakHitResult` _outhit))))
                (set `self.Landscape` _aslandscape)
                (if (and (== _landscape (`.HitActor` (`GameplayStatics.BreakHitResult` _outhit))) _returnvalue_4)
                  (bind (_canvas _size _context) (`KismetRenderingLibrary.BeginDrawCanvasToRenderTarget` "/Game/Dynamic_landscape/Dynamic_render_target.Dynamic_render_target"))
                  (bind (_returnvalue_x_4 _returnvalue_y_3) (`KismetMathLibrary.BreakVector2D` (- (`KismetMathLibrary.MakeVector2D` _returnvalue_x_2 _returnvalue_y_2) (`KismetMathLibrary.MakeVector2D` (.x (`.Location` (`GameplayStatics.BreakHitResult` _outhit))) (.y (`.Location` (`GameplayStatics.BreakHitResult` _outhit)))))))
                  (bind (_screen_position _screen_size) (`/Engine/ArtTools/RenderToTexture/Macros/RenderToTextureFunctionLibrary.Set Canvas Material Scale and Position` _size (`KismetMathLibrary.MakeVector2D` (/ (`KismetMathLibrary.Abs` _returnvalue_x_4) (* (.x _boxextent) 2.0)) (/ (`KismetMathLibrary.Abs` _returnvalue_y_3) (* (.y _boxextent) 2.0))) (* _returnvalue_x_3 20.0)))
                  (`Canvas.K2_DrawMaterial` _canvas (`self.Render Material`) _screen_position _screen_size (0.0 0.0) (1.0 1.0) 0.0 (0.5 0.5))
                  (`KismetRenderingLibrary.EndDrawCanvasToRenderTarget` _context))
                (elif (< _returnvalue_x -8000.0)
                  (goto _label)
                  (else
                    (`self.SetActorHiddenInGame` true :!label _label_2)
                    (`self.K2_SetActorLocation` (`KismetMathLibrary.MakeVector` _returnvalue_2 _returnvalue_3 10000.0))))))
            (:`then_1`
              (if (> _returnvalue_y 8000.0)
                (goto _label)
                (elif (< _returnvalue_y -8000.0)
                  (goto _label)
                  (else
                    (goto _label_2))))))
          (else
            (goto _label_2)))
        (else
          (goto _label_2)))
      (else
        (goto _label_2)))
    (else
      (goto _label_2))))

(fn `UserConstructionScript`)