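; Interactive wooden door that opens on E and swings shut by itself after a few seconds.
; A box overlap enables input for the first-person character, and a gated per-tick loop records how long E is held.
; On release, a hold past the threshold opens the door at normal speed, while a shorter press opens it faster.
; Timelines turn the handle, then rotate the door after a brief delay and later reverse it.
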(event `HandleAnim`
  (bind (_direction _alpha) (`Timeline|Timeline_0` :!via `PlayFromStart`)
    (:`Update`
      (`SceneComponent.K2_SetRelativeRotation` (`self.HandleRotatePoint`) (`KismetMathLibrary.RLerp` (struct) (struct :`Pitch` -60.0) _alpha) false false))))

(event `RunTimeline`
  (if (not (`self.Opening`))
    (`|ExecutionSequence`
      (:`then_0`
        (set `self.Opening` true)
        (`self.HandleAnim`)
        (`KismetSystemLibrary.Delay` 0.3)
        (bind (_direction _alpha) (`Timeline|TL_DoorRotate` :!label _label)
          (:`Update`
            (`SceneComponent.K2_SetRelativeRotation` (`self.RotatePoint`) (`KismetMathLibrary.RLerp` (struct) (`self.Open Angle`) _alpha) false false))))
      (:`then_1`
        (`KismetSystemLibrary.Delay` 4.0)
        (set `self.Opening` false)
        (goto _label :!via `Reverse`)))))

(event `self.Box.OnComponentBeginOverlap`
  (params (OverlappedComponent :type "PrimitiveComponent Object Reference") (OtherActor :type "Actor Object Reference") (OtherComp :type "PrimitiveComponent Object Reference") (OtherBodyIndex :type Integer) (bFromSweep :type Boolean) (SweepResult :type "HitResult Structure (by ref)"))
  (cast `/Game/MOUT_Fabrication/Demo/FirstPersonBP/Blueprints/FirstPersonCharacter` OtherActor)
  (`self.EnableInput` (`GameplayStatics.GetPlayerController` 0)))

(event `self.Box.OnComponentEndOverlap`
  (params (OverlappedComponent :type "PrimitiveComponent Object Reference") (OtherActor :type "Actor Object Reference") (OtherComp :type "PrimitiveComponent Object Reference") (OtherBodyIndex :type Integer))
  (cast `/Game/MOUT_Fabrication/Demo/FirstPersonBP/Blueprints/FirstPersonCharacter` OtherActor)
  (`self.DisableInput` (`GameplayStatics.GetPlayerController` 0)))

(event `Key|E`
  (params (Key :type "Key Structure"))
  (bind _tl_doorrotate (`self.TL_DoorRotate`))
  (:`Pressed`
    (`|ExecutionSequence`
      (:`then_0`
        (goto _label_2 :!via `Open`))
      (:`then_1`
        (`/Engine/EditorBlueprintResources/StandardMacros.Gate` false :!label _label_2
          (:`Exit`
            (bind _output_get (set `self.KeyPressedTime` (`PlayerController.GetInputKeyTimeDown` (`GameplayStatics.GetPlayerController` 0) Key)))
            (`KismetSystemLibrary.Delay` 0.0)
            (goto _label_2))))))
  (:`Released`
    (`|ExecutionSequence`
      (:`then_0`
        (goto _label_2 :!via `Close`))
      (:`then_1`
        (if (>= _output_get (`self.Hold Down Time`))
          (`TimelineComponent.SetPlayRate` _tl_doorrotate 1.0)
          (`self.RunTimeline`)
          (else
            (`TimelineComponent.SetPlayRate` _tl_doorrotate 4.0)
            (`self.RunTimeline`)))))))

(fn `UserConstructionScript`)