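; BP_HalfTarget_Stand02 is a target stand that rotates when the first-person character enters its trigger box.
; Overlap plays a timeline that lerps the RotatePoint's relative rotation from a 90-degree tilt to zero.
; When the character leaves, the timeline reverses after a configurable delay.
; The construction script applies an exposed transform to the trigger box, so its placement can differ from the stand's.
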(event `self.TriggerBox.OnComponentBeginOverlap`
  (params (OverlappedComponent :type "PrimitiveComponent Object Reference") (OtherActor :type "Actor Object Reference") (OtherComp :type "PrimitiveComponent Object Reference") (OtherBodyIndex :type Integer) (bFromSweep :type Boolean) (SweepResult :type "HitResult Structure (by ref)"))
  (cast `/Game/MOUT_Fabrication/Demo/FirstPersonBP/Blueprints/FirstPersonCharacter` OtherActor)
  (bind (_direction _alpha) (`Timeline|TL_TargetRotate` :!label _label)
    (:`Update`
      (`SceneComponent.K2_SetRelativeRotation` (`self.RotatePoint`) (`KismetMathLibrary.RLerp` (struct :`Roll` 90.0) (struct) _alpha) false false))))

(event `self.TriggerBox.OnComponentEndOverlap`
  (params (OverlappedComponent :type "PrimitiveComponent Object Reference") (OtherActor :type "Actor Object Reference") (OtherComp :type "PrimitiveComponent Object Reference") (OtherBodyIndex :type Integer))
  (cast `/Game/MOUT_Fabrication/Demo/FirstPersonBP/Blueprints/FirstPersonCharacter` OtherActor)
  (`KismetSystemLibrary.Delay` (`self.Duration`))
  (goto _label :!via `Reverse`))

(fn `UserConstructionScript`
  (`SceneComponent.K2_SetRelativeTransform` (`self.TriggerBox`) (`self.TriggerBoxTransform`) false false))