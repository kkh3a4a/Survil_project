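; An interactable barrier gate that the first-person character opens with the E key and that closes automatically.
; A box overlap enables and disables player input on the actor.
; Pressing E while closed plays timelines that slide the lock and then rotate the gate toward OpenAngle.
; Chained delays then reverse both timelines and restore the IsClosed flag, which blocks re-triggering during the cycle.
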(event `LockOpen`
  (bind (_direction _alpha) (`Timeline|TL_Lock` :!label _label)
    (:`Update`
      (`SceneComponent.K2_SetRelativeLocation` (`self.Lock`) (`KismetMathLibrary.VLerp` (0.0 0.0 0.0) (-6.0 0.0 0.0) _alpha) false false))))

(event `LockClose`
  (goto _label :!via `Reverse`))

(event `GateOpen`
  (bind (_direction _alpha) (`Timeline|OpenGate` :!label _label_2)
    (:`Update`
      (`SceneComponent.K2_SetRelativeRotation` (`self.RotatePoint`) (`KismetMathLibrary.RLerp` (struct) (`self.Open Angle`) _alpha) false false))))

(event `GateClose`
  (goto _label_2 :!via `Reverse`))

(event `Key|E`
  (params (Key :type "Key Structure"))
  (:`Pressed`
    (if (`self.IsClosed`)
      (`|ExecutionSequence`
        (:`then_0`
          (set `self.IsClosed` false)
          (`self.LockOpen`))
        (:`then_1`
          (`KismetSystemLibrary.Delay` 1.0)
          (`self.GateOpen`)
          (`KismetSystemLibrary.Delay` 5.0)
          (`self.GateClose`)
          (`KismetSystemLibrary.Delay` 2.5)
          (`|ExecutionSequence`
            (:`then_0`
              (`self.LockClose`))
            (:`then_1`
              (`KismetSystemLibrary.Delay` 1.0)
              (set `self.IsClosed` true))))))))

(event `self.Box.OnComponentBeginOverlap`
  (params (OverlappedComponent :type "PrimitiveComponent Object Reference") (OtherActor :type "Actor Object Reference") (OtherComp :type "PrimitiveComponent Object Reference") (OtherBodyIndex :type Integer) (bFromSweep :type Boolean) (SweepResult :type "HitResult Structure (by ref)"))
  (cast `/Game/MOUT_Fabrication/Demo/FirstPersonBP/Blueprints/FirstPersonCharacter` OtherActor)
  (`self.EnableInput` (`GameplayStatics.GetPlayerController` 0)))

(event `self.Box.OnComponentEndOverlap`
  (params (OverlappedComponent :type "PrimitiveComponent Object Reference") (OtherActor :type "Actor Object Reference") (OtherComp :type "PrimitiveComponent Object Reference") (OtherBodyIndex :type Integer))
  (cast `/Game/MOUT_Fabrication/Demo/FirstPersonBP/Blueprints/FirstPersonCharacter` OtherActor)
  (`self.DisableInput` (`GameplayStatics.GetPlayerController` 0)))

(fn `UserConstructionScript`)