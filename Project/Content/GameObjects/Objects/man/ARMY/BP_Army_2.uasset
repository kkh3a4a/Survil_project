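; BP_Army_2 is an army unit actor that displays a health bar and removes itself when dead.
; On BeginPlay it spawns a separate CharHpBar actor at its DummyHP component with a fixed rotation and disables the bar widget's shadow.
; Each Tick moves the bar to DummyHP, refreshes it from ArmyHP, and calls IsDead, which destroys both actors when State equals 3.
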(event `self.ReceiveBeginPlay`
  (bind _returnvalue (`|SpawnActorFromClass` "/Game/UI/Widget/InGame_widget/CharHpBar.CharHpBar_C" (`KismetMathLibrary.MakeTransform` (`SceneComponent.K2_GetComponentLocation` (`self.DummyHP`)) (struct :`Pitch` 45.0 :`Yaw` 90.0)) "Undefined" "OverrideRootScale" null null))
  (bind _output_get (set `self.HP_Actor` _returnvalue))
  ;[1 1 1] HP bar 그림자 삭제
  (`PrimitiveComponent.SetCastShadow` (`/Game/UI/Widget/InGame_widget/CharHpBar.Widget` _output_get) false))

(event `self.ReceiveTick`
  (params (DeltaSeconds :type "Float (single-precision)"))
  (`/Game/UI/Widget/InGame_widget/CharHpBar.UpdateLocation` (`self.HP_Actor`) (`SceneComponent.K2_GetComponentLocation` (`self.DummyHP`)))
  (`/Game/UI/Widget/InGame_widget/CharHpBar.UpdateHp` (`self.HP_Actor`) 100.0 (`self.Army_HP`))
  (`self.Is_Dead` (`self.state`)))

(fn `Dead`)

(fn `Is_Dead`
  (params (NewParam :type Byte))
  (if (== NewParam 3)
    (`self.K2_DestroyActor` (`self.HP_Actor`))
    (`self.K2_DestroyActor`)))

(fn `UserConstructionScript`)